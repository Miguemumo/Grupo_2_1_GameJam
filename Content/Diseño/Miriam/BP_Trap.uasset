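; BP_Trap is a trap actor that switches between open and closed by rotating its two parts.
; The TrapStart event flips the Opened flag, and BeginPlay applies that flag's initial state.
; Both events call GetNewRotation on each part, which instantly snaps its relative roll between upright and a quarter turn while keeping pitch and yaw.
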(event Custom|TrapStart
  (bind _output_get (Variables|Default|SetOpened (not (Variables|Default|GetOpened))))
  (CallFunction|GetNewRotation (Variables|Default|GetBP_TrapPart) _output_get)
  (CallFunction|GetNewRotation (Variables|Default|GetBP_TrapPart1) _output_get))

(event EventBeginPlay
  (bind _opened (Variables|Default|GetOpened))
  (CallFunction|GetNewRotation (Variables|Default|GetBP_TrapPart) _opened)
  (CallFunction|GetNewRotation (Variables|Default|GetBP_TrapPart1) _opened))

(fn ConstructionScript)

(fn GetNewRotation
  (params (Element :type Scene%20Component%20Object%20Reference) (Opened :type Boolean))
  (bind _relativerotation (Variables|/Script/Engine.SceneComponent|GetRelativeRotation Element))
  (Transformation|SetRelativeRotation Element (Math|Rotator|MakeRotator (Math|Float|SelectFloat 9e+01 0.0 Opened) (.pitch _relativerotation) (.yaw _relativerotation)) false false))