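; BP_CompressSlime squashes and restores its owning actor, presumably a slime, and caches that owner on BeginPlay.
; GetDownSlime halves the owner's Z scale and GetSlimeBack resets it to full scale, both instantly through SetActorTransform with unchanged location and rotation.
; Each event also updates the IsCompressed flag to record the current state.
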(event Custom|GetDownSlime
  (bind _owner (Variables|Default|GetOwner))
  (Transformation|SetActorTransform _owner (Math|Transform|MakeTransform (Transformation|GetActorLocation _owner) (Transformation|GetActorRotation _owner) "1,1,0.500000"))
  (Variables|Default|SetIsCompressed true))

(event Custom|GetSlimeBack
  (bind _owner (Variables|Default|GetOwner))
  (Transformation|SetActorTransform _owner (Math|Transform|MakeTransform (Transformation|GetActorLocation _owner) (Transformation|GetActorRotation _owner) "1,1,1.000000"))
  (Variables|Default|SetIsCompressed false))

(event EventBeginPlay
  (Variables|Default|SetOwner (Components|GetOwner)))

(event EventTick
  (params (DeltaSeconds :type Float%20%28single-precision%29)))