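; BP_Enemy is an enemy that chases pawns it sees and can be destroyed by the player.
; On begin play it applies its Speed to walking, and PawnSensing triggers simple moves toward the seen pawn's current location.
; When BP_Character overlaps the Box, the enemy is destroyed and launches that character upward, like a stomp bounce.
; When BP_Character hits the capsule instead, it creates and shows the WBP_GameOver widget.
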(event OnSeePawn(PawnSensing)
  (params (Pawn :type Pawn%20Object%20Reference))
  (AI|Navigation|SimpleMovetoLocation (Pawn|GetController) (Transformation|GetActorLocation Pawn)))

(event OnComponentBeginOverlap(Box)
  (params (OverlappedComponent :type Primitive%20Component%20Object%20Reference) (OtherActor :type Actor%20Object%20Reference) (OtherComp :type Primitive%20Component%20Object%20Reference) (OtherBodyIndex :type Integer) (bFromSweep :type Boolean) (SweepResult :type Hit%20Result%20Structure%20%28by%20ref%29))
  (bind _asbp_character (Utilities|Casting|CastToBP_Character OtherActor))
  (Actor|DestroyActor)
  (Character|LaunchCharacter _asbp_character "0, 0,600.000000" false true))

(event OnComponentHit(CapsuleComponent)
  (params (HitComponent :type Primitive%20Component%20Object%20Reference) (OtherActor :type Actor%20Object%20Reference) (OtherComp :type Primitive%20Component%20Object%20Reference) (NormalImpulse :type Vector :default "0, 0, 0") (Hit :type Hit%20Result%20Structure%20%28by%20ref%29))
  (Utilities|Casting|CastToBP_Character OtherActor)
  (bind _returnvalue (UserInterface|CreateWidget "/Game/Blueprints/Widget/WBP_GameOver.WBP_GameOver_C"))
  (UserInterface|Viewport|AddtoViewport _returnvalue 0))

(event EventBeginPlay
  (Variables|/Script/Engine.CharacterMovementComponent|SetMaxWalkSpeed (Variables|Character|GetCharacterMovement) (Variables|Default|GetSpeed)))

(fn ConstructionScript)